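; Wizard ice barrier that sizes itself to surrounding geometry and blocks projectiles.
; Raycast traces along the spawner's orientation to fit the box, derives health from size (larger is weaker) and charges mana.
; A looping timer rotates, then moves and scales the wall into place; unfinished barriers expire after a delay.
; Overlapping projectiles are destroyed and drain health, shown through a dynamic material, until the barrier is destroyed.
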(event OnComponentBeginOverlap(Box)
  (params (OverlappedComponent :type Primitive%20Component%20Object%20Reference) (OtherActor :type Actor%20Object%20Reference) (OtherComp :type Primitive%20Component%20Object%20Reference) (OtherBodyIndex :type Integer) (bFromSweep :type Boolean) (SweepResult :type Hit%20Result%20Structure%20%28by%20ref%29))
  (bind _asprojectile_hit_box (Utilities|Casting|CastToProjectileHitBox OtherActor))
  (Default|Destroy _asprojectile_hit_box)
  (CallFunction|DecrementHealth 1e+01))

(event OnComponentEndOverlap(Box)
  (params (OverlappedComponent :type Primitive%20Component%20Object%20Reference) (OtherActor :type Actor%20Object%20Reference) (OtherComp :type Primitive%20Component%20Object%20Reference) (OtherBodyIndex :type Integer)))

(event Custom|Raycast
  (bind _forwardvector (Variables|Default|GetForwardVector))
  (bind _box (Variables|Default|GetBox))
  (bind _forwardvector_2 (Variables|Default|GetForwardVector))
  (bind _box_2 (Variables|Default|GetBox))
  (bind _returnvalue (Math|Vector|GetRightVector _forwardvector))
  (bind _returnvalue_2 (Transformation|GetWorldRotation _forwardvector_2))
  (bind _returnvalue_3 (Components|Box|GetScaledBoxExtent _box_2))
  (bind _returnvalue_4 (/ (.y _returnvalue_3) 96.0))
  ;[1 1 1] Init Plane Scale
  (Transformation|SetWorldScale3D (Variables|Default|GetWall) (Math|Vector|MakeVector _returnvalue_4 _returnvalue_4 _returnvalue_4))
  ;[1 1 1] Rotate Raycast Dirs to Player Forward Vec
  (Transformation|SetWorldRotation (Variables|Default|GetForwardVector) (Transformation|GetWorldRotation (Variables|/Script/Engine.Character|GetCapsuleComponent (Variables|Default|GetSpawner))) false false)
  ;[1 1 1] Do Raycast to Surroundings
  (bind (_length _midpoint) (CallFunction|GetLineMidpointandLength (Math|Vector|GetUpVector (Variables|Default|GetForwardVector))))
  (bind _output_get (Variables|Default|SetHeight _length))
  (bind (_length_2 _midpoint_2) (CallFunction|GetLineMidpointandLength _returnvalue))
  (bind _output_get_2 (Variables|Default|SetWidth _length_2))
  (if (or (< _output_get_2 5.0) (< _output_get 5.0))
    (Actor|DestroyActor)
    (else
      ;[1 1 1] Set Collision Box Extents from Raycast
      (Components|Box|SetBoxExtent _box (Math|Vector|MakeVector (Variables|Default|GetHeight) (Variables|Default|GetWidth) 1e+02) true)
      ;[1 1 1] Move Collision Box to Center And Rotate to Player's Rot
      (Transformation|SetWorldLocationAndRotation _box (Math|Vector|FindClosestPointonLine _midpoint_2 _midpoint _returnvalue) (Math|Rotator|MakeRotator (.roll _returnvalue_2) 9e+01 (.yaw _returnvalue_2)) false false)
      (Variables|Default|SetDesiredPlaneRotation (Math|Rotator|MakeRotator (.roll _returnvalue_2) 9e+01 (.yaw _returnvalue_2)))
      ;[1 1 1] Set Desired Plane scale
      (Variables|Default|SetDesiredPlaneScale (Math|Vector|MakeVector (/ (Variables|Default|GetHeight) 96.0) (/ (Variables|Default|GetWidth) 96.0) 1.0))
      (Variables|Default|SetDesiredPlaneLocation (Math|Vector|FindClosestPointonLine _midpoint_2 _midpoint _returnvalue))
      (bind _output_get_3 (Variables|Default|SetBarrierHealth (/ (- 5e+03 (+ (Variables|Default|GetHeight) (Variables|Default|GetWidth))) 5e+01)))
      (Default|DecrementMana (Variables|Default|GetSpawner) (+ (/ _output_get_3 2.0) 1e+01))
      (bind _returnvalue_5 (Rendering|Material|CreateDynamicMaterialInstance (Rendering|Material|GetMaterial (Variables|Default|GetWall) 0) "None" "None" :!class /Script/Engine.KismetMaterialLibrary))
      (bind _output_get_4 (Variables|Default|SetDynamicMaterial _returnvalue_5))
      (Rendering|Material|SetMaterial (Variables|Default|GetWall) 0 _output_get_4)
      (Rendering|Material|SetScalarParameterValue _output_get_4 "BarrierHealth" (Math|Float|Clamp(Float) (/ (Variables|Default|GetBarrierHealth) 1e+02) 0.1) :!class /Script/Engine.MaterialInstanceDynamic)
      (bind _returnvalue_6 (Utilities|Time|SetTimerbyFunctionName 0 "InterpPlaneToDesired" 0.05 true 0.5 0.3))
      (Variables|Default|SetInterpTimer _returnvalue_6))))

(event EventBeginPlay
  (Utilities|FlowControl|Delay 8.0)
  (if (not (Variables|Default|GetIsDone))
    (Actor|DestroyActor)))

(fn ConstructionScript)

(fn GetLineMidpointandLength
  (params (Direction :type Vector))
  (bind _returnvalue (Transformation|GetActorLocation))
  (bind _returnvalue_2 (Transformation|GetActorLocation))
  (bind _outhit (Collision|LineTraceByChannel _returnvalue_2 (+ _returnvalue_2 (* Direction (Variables|Default|GetRaycastDist))) "TraceTypeQuery2" false 0 "None"))
  (LocalVariables|SetHitLoc1 (.location _outhit))
  (LocalVariables|SetIsHit (.bblockinghit _outhit))
  (bind _outhit_2 (Collision|LineTraceByChannel _returnvalue_2 (+ _returnvalue_2 (* Direction (* (Variables|Default|GetRaycastDist) -1.0))) "TraceTypeQuery2" false 0 "None"))
  (LocalVariables|SetIsHit (or (.bblockinghit _outhit_2) (LocalVariables|GetIsHit)))
  (LocalVariables|SetHitLoc2 (.location _outhit_2))
  (if (Utilities|Operators|EqualEqual :A (LocalVariables|GetHitLoc1))
    (LocalVariables|SetHitLoc1 (+ _returnvalue (* Direction 5e+02))))
  (if (Utilities|Operators|EqualEqual :A (LocalVariables|GetHitLoc2))
    (LocalVariables|SetHitLoc2 (+ _returnvalue (* Direction -5e+02))))
  (if (LocalVariables|GetIsHit)
    (LocalVariables|Set_midpoint (+ (LocalVariables|GetHitLoc2) (* (Math|Vector|Normalize (- (LocalVariables|GetHitLoc1) (LocalVariables|GetHitLoc2))) (/ (Math|Vector|VectorLength (- (LocalVariables|GetHitLoc1) (LocalVariables|GetHitLoc2))) 2.0))))
    (else
      (LocalVariables|Set_midpoint (Transformation|GetActorLocation))))
  (return (Math|Vector|Distance(Vector) (LocalVariables|GetHitLoc2) (LocalVariables|GetHitLoc1)) (+ (LocalVariables|GetHitLoc2) (* (Math|Vector|Normalize (- (LocalVariables|GetHitLoc1) (LocalVariables|GetHitLoc2))) (/ (Math|Vector|VectorLength (- (LocalVariables|GetHitLoc1) (LocalVariables|GetHitLoc2))) 2.0)))))

(fn DecrementHealth
  (params (DmgAmt :type Float%20%28double-precision%29))
  (bind _output_get (Variables|Default|SetBarrierHealth (- (Variables|Default|GetBarrierHealth) DmgAmt)))
  (Rendering|Material|SetScalarParameterValue (Variables|Default|GetDynamicMaterial) "BarrierHealth" (Math|Float|Clamp(Float) (/ _output_get 1e+02) 0.1) :!class /Script/Engine.MaterialInstanceDynamic)
  (if (< (Variables|Default|GetBarrierHealth) 0.0)
    (Actor|DestroyActor)))

(fn InterpPlanetoDesired
  (bind _returnvalue (Utilities|Time|GetWorldDeltaSeconds))
  (bind _wall (Variables|Default|GetWall))
  (bind _wall_2 (Variables|Default|GetWall))
  (if (Variables|Default|GetIsRotated)
    (Transformation|SetWorldTransform _wall (Math|Transform|MakeTransform (Math|Interpolation|VInterpTo (Transformation|GetWorldLocation _wall) (Variables|Default|GetDesiredPlaneLocation) _returnvalue 5.0) (Math|Interpolation|RInterpTo (Transformation|GetWorldRotation _wall) (Variables|Default|GetDesiredPlaneRotation) _returnvalue 1e+01) (Math|Interpolation|VInterpTo (Transformation|GetWorldScale _wall) (Variables|Default|GetDesiredPlaneScale) _returnvalue 5.0)) false false)
    (if (Class|KismetMathLibrary|NearlyEqualTransformTransform (Transformation|GetWorldTransform (Variables|Default|GetWall)) (Math|Transform|MakeTransform (Variables|Default|GetDesiredPlaneLocation) (Variables|Default|GetDesiredPlaneRotation) (Variables|Default|GetDesiredPlaneScale)) 2.0 2.0 0.0)
      (Variables|Default|SetIsDone true)
      (Development|PrintString "INTERP")
      (Utilities|Time|ClearandInvalidateTimerbyHandle (Variables|Default|GetInterpTimer))
      (Components|DestroyComponent (Variables|Default|GetNiagara9)))
    (else
      (Transformation|SetWorldTransform _wall_2 (Math|Transform|MakeTransform (Transformation|GetWorldLocation _wall_2) (Math|Interpolation|RInterpTo (Transformation|GetWorldRotation _wall_2) (Variables|Default|GetDesiredPlaneRotation) (Utilities|Time|GetWorldDeltaSeconds) 1e+01) (Transformation|GetWorldScale _wall_2)) false false)
      (if (Utilities|Operators|EqualEqual (Transformation|GetWorldRotation (Variables|Default|GetWall)) (Variables|Default|GetDesiredPlaneRotation) 2.0)
        (Variables|Default|SetIsRotated true)))))
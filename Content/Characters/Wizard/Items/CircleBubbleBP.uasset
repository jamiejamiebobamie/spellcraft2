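; CircleBubbleBP is a timed bubble in the wizard's items that captures actors implementing Circleable.
; Sphere overlap claims valid, uncircled Circleables, tracks them in an array and attaches actors keeping world transforms, while end overlap resets their circled state and untracks them.
; Tick applies force to each valid tracked Circleable.
; After Lifespan, PopBubble resets the circled state of those still owned by this bubble and destroys itself.
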(event OnComponentBeginOverlap(Sphere)
  (params (OverlappedComponent :type Primitive%20Component%20Object%20Reference) (OtherActor :type Actor%20Object%20Reference) (OtherComp :type Primitive%20Component%20Object%20Reference) (OtherBodyIndex :type Integer) (bFromSweep :type Boolean) (SweepResult :type Hit%20Result%20Structure%20%28by%20ref%29))
  (bind _ascircleable (Utilities|Casting|CastToCircleable OtherActor))
  (bind _returnvalue (Class|Circleable|GetIsValid _ascircleable))
  (if _returnvalue
    (bind _returnvalue_2 (Class|Circleable|GetIsCircled _ascircleable))
    (if (not (Utilities|IsValid _returnvalue_2))
      (Class|Circleable|SetIsCircled _ascircleable)
      (Utilities|Array|Add (Variables|Default|GetCircleables) _ascircleable)
      (Transformation|AttachActorToActor self 0 "None" "KeepWorld" "KeepWorld" "KeepWorld" true))))

(event OnComponentEndOverlap(Sphere)
  (params (OverlappedComponent :type Primitive%20Component%20Object%20Reference) (OtherActor :type Actor%20Object%20Reference) (OtherComp :type Primitive%20Component%20Object%20Reference) (OtherBodyIndex :type Integer))
  (bind _ascircleable (Utilities|Casting|CastToCircleable OtherActor))
  (bind _returnvalue (Class|Circleable|GetIsValid _ascircleable))
  (if _returnvalue
    (if (Utilities|Array|ContainsItem (Variables|Default|GetCircleables) _ascircleable)
      (Class|Circleable|SetIsCircled _ascircleable)
      (Utilities|Array|RemoveItem (Variables|Default|GetCircleables) _ascircleable))))

(event EventBeginPlay
  (Utilities|FlowControl|Delay (Variables|Default|GetLifespan))
  (CallFunction|PopBubble))

(event EventTick
  (params (DeltaSeconds :type Float%20%28single-precision%29))
  (for _array_element (Variables|Default|GetCircleables)
    (bind _returnvalue (Class|Circleable|GetIsValid _array_element))
    (if _returnvalue
      (Class|Circleable|ApplyForce _array_element))))

(fn ConstructionScript)

(fn PopBubble
  (for _array_element (Variables|Default|GetCircleables)
    (bind _returnvalue (Class|Circleable|GetIsCircled _array_element))
    (if (== _returnvalue self)
      (Class|Circleable|SetIsCircled _array_element)))
  (Actor|DestroyActor))
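; Wizard Circle spell bubble that captures overlapping Circleable objects and floats them upward until it pops.
; It implements Circleable itself, self-registers, claims unowned objects entering its sphere, and releases them on exit.
; Tick applies upward force to everything held, and impulses on the bubble pass scaled force to its contents.
; A resettable lifespan timer calls PopBubble to free contents, spawn Niagara and destroy it, whereas Damage destroys it directly.
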(event OnComponentHit(Sphere)
  (params (HitComponent :type Primitive%20Component%20Object%20Reference) (OtherActor :type Actor%20Object%20Reference) (OtherComp :type Primitive%20Component%20Object%20Reference) (NormalImpulse :type Vector :default "0, 0, 0") (Hit :type Hit%20Result%20Structure%20%28by%20ref%29)))

(event OnComponentBeginOverlap(Sphere)
  (params (OverlappedComponent :type Primitive%20Component%20Object%20Reference) (OtherActor :type Actor%20Object%20Reference) (OtherComp :type Primitive%20Component%20Object%20Reference) (OtherBodyIndex :type Integer) (bFromSweep :type Boolean) (SweepResult :type Hit%20Result%20Structure%20%28by%20ref%29))
  (if (!= OtherActor self)
    (bind _ascircleable (Utilities|Casting|CastToCircleable OtherActor))
    (bind _returnvalue (Class|Circleable|GetIsValid _ascircleable))
    (if _returnvalue
      (bind _returnvalue_2 (Class|Circleable|GetIsCircled _ascircleable))
      (if (not (Utilities|IsValid _returnvalue_2))
        (Class|Circleable|SetIsCircled _ascircleable self)
        (Utilities|Array|Add (Variables|Default|GetCircleables) _ascircleable)))))

(event OnComponentEndOverlap(Sphere)
  (params (OverlappedComponent :type Primitive%20Component%20Object%20Reference) (OtherActor :type Actor%20Object%20Reference) (OtherComp :type Primitive%20Component%20Object%20Reference) (OtherBodyIndex :type Integer))
  (if (!= OtherActor self)
    (bind _ascircleable (Utilities|Casting|CastToCircleable OtherActor))
    (bind _returnvalue (Class|Circleable|GetIsValid _ascircleable))
    (if _returnvalue
      (if (Utilities|Array|ContainsItem (Variables|Default|GetCircleables) _ascircleable)
        (Class|Circleable|SetIsCircled _ascircleable)
        (Utilities|Array|RemoveItem (Variables|Default|GetCircleables) _ascircleable)))))

(event EventBeginPlay
  (Utilities|FlowControl|Sequence
    (:then_0
      (bind _ascircleable (Utilities|Casting|CastToCircleable self))
      (CallFunction|SetIsCircled _ascircleable self)
      (Utilities|Array|Add (Variables|Default|GetCircleables) _ascircleable))
    (:then_1
      (Class|CircleBubble|SetBubbleLifespan (Variables|Default|GetDefaultBubbleLifespan)))))

(event EventTick
  (params (DeltaSeconds :type Float%20%28single-precision%29))
  (for _array_element (Variables|Default|GetCircleables)
    (bind _returnvalue (Class|Circleable|GetIsValid _array_element))
    (if _returnvalue
      (Class|Circleable|ApplyForce _array_element "0.000000,0.000000,1.000000"))))

(event EventSetBubbleLifespan
  (params (seconds :type Float%20%28single-precision%29))
  (Utilities|Time|ClearandInvalidateTimerbyHandle (Variables|Default|GetSetBubbleLifespanTimer))
  (bind _returnvalue (Utilities|Time|SetTimerbyFunctionName 0 "PopBubble" seconds))
  (Variables|Default|SetSetBubbleLifespanTimer _returnvalue))

(fn ConstructionScript)

(fn PopBubble
  (for _array_element (Variables|Default|GetCircleables)
    (bind _returnvalue (Class|Circleable|GetIsCircled _array_element))
    (if (== _returnvalue self)
      (Class|Circleable|SetIsCircled _array_element)))
  (Niagara|SpawnSystematLocation "/Game/Characters/Wizard/Effects/AdvancedMagicFX12/particles/Niagara/NS_ky_hit_bubble.NS_ky_hit_bubble" (Transformation|GetActorLocation))
  (Actor|DestroyActor))

(fn GetLocation
  (return (Transformation|GetActorLocation)))

(fn ApplyImpulse
  (params (Impulse :type Vector :default "0, 0, 0"))
  (for _array_element (Variables|Default|GetCircleables)
    (Class|Circleable|ApplyForce _array_element (/ Impulse 18.0)))
  (Physics|AddImpulse (Variables|Default|GetSphere) Impulse "None" false)
  (return true))

(fn SetIsCircled
  (params (CircleBubble :type Circle%20Bubble%20Object%20Reference))
  (Variables|Circleable|SetCircleBubble CircleBubble)
  (return true))

(fn GetIsValid
  (return (Utilities|IsValid self)))

(fn ApplyForce
  (params (OptionalForce :type Vector :default "0, 0, 0"))
  (if (Utilities|IsValid self)
    (Physics|AddForce (Variables|Default|GetSphere) (Math|Vector|MakeVector 0.0 0.0 1e+03) "None" false)
    (return true)))

(fn GetIsCircled
  (return (Variables|Circleable|GetCircleBubble)))

(fn Damage
  (params (dmgAmt :type Float%20%28single-precision%29))
  (Actor|DestroyActor)
  (return true))

(fn SpawnHitParticle
  (params (Particle :type Niagara%20System%20Object%20Reference) (HitNormal :type Vector :default "0, 0, 0") (Location :type Vector :default "0, 0, 0"))
  (Niagara|SpawnSystematLocation "/Game/Characters/Wizard/Effects/AdvancedMagicFX12/particles/Niagara/NS_ky_hit_bubble.NS_ky_hit_bubble" (Transformation|GetActorLocation))
  (return false))
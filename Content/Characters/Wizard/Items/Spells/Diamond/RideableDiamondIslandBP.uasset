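; Rideable diamond island spell actor for the Wizard, which carries a flying rider until it hits something.
; SetIsRiding arms collision dismounting after a one-second delay, so overlaps before then are ignored.
; Once armed, any island overlap with an actor other than the rider calls Dismount.
; Dismount restores a valid rider's default targeting distance and walking movement, clears flying, then destroys the island.
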(event OnComponentBeginOverlap(Island)
  (params (OverlappedComponent :type Primitive%20Component%20Object%20Reference) (OtherActor :type Actor%20Object%20Reference) (OtherComp :type Primitive%20Component%20Object%20Reference) (OtherBodyIndex :type Integer) (bFromSweep :type Boolean) (SweepResult :type Hit%20Result%20Structure%20%28by%20ref%29))
  ;[1 1 1] Player hit something
  (if (Variables|Default|GetIsRiding)
    (if (!= (Variables|Default|GetRider) OtherActor)
      (CallFunction|Dismount))))

(event Custom|SetIsRiding
  (Utilities|FlowControl|Delay 1.0)
  (Variables|Default|SetIsRiding true))

(fn ConstructionScript)

(fn Dismount
  (if (Utilities|IsValid (Variables|Default|GetRider))
    (Default|SetTargetableMaxDistancetoDefault (Variables|Default|GetRider))
    (Variables|/Game/Characters/Wizard/WizardBaseBP.WizardBaseBP_C|SetIsFlying (Variables|Default|GetRider) false)
    (Pawn|Components|CharacterMovement|SetMovementMode (Variables|/Script/Engine.Character|GetCharacterMovement (Variables|Default|GetRider)) "MOVE_Walking" 0))
  (Actor|DestroyActor))
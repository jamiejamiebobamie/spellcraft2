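; Wizard Diamond spell island that drops after a short delay, damages Damageable actors by its scale on impact, and destroys itself on hitting anything but another island.
; SetIsCircled with a valid bubble suspends falling, overrides mass and damping, and adds a rider-detection sphere.
; While the Spawner overlaps it, a looping timer debug-traces a predicted launch toward RiderConnectionPoint when the camera faces it, without launching anyone.
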(event OnComponentHit(Island)
  (params (HitComponent :type Primitive%20Component%20Object%20Reference) (OtherActor :type Actor%20Object%20Reference) (OtherComp :type Primitive%20Component%20Object%20Reference) (NormalImpulse :type Vector :default "0, 0, 0") (Hit :type Hit%20Result%20Structure%20%28by%20ref%29))
  (bind _island (Variables|Default|GetIsland))
  (bind _dmgmultiplier (Variables|Default|GetDmgMultiplier))
  (bind _returnvalue (Transformation|GetWorldScale _island))
  (bind _returnvalue_2 (Math|Vector|VectorLength _returnvalue))
  (bind _returnvalue_3 (* _returnvalue_2 _dmgmultiplier))
  (if (Variables|Default|GetIsFalling)
    (Utilities|Casting|CastToDiamondIsland OtherActor
      (:CastFailed
        (bind _asdamageable (Utilities|Casting|CastToDamageable OtherActor)
          (:then
            (Development|PrintString (Utilities|String|ToString(Float) _returnvalue_3))
            (Class|Damageable|Damage _asdamageable _returnvalue_3))
          (:CastFailed
            _))
        (Actor|DestroyActor)))))

(event Custom|CheckForRider
  (params (OverlappedComponent :type Primitive%20Component%20Object%20Reference) (OtherActor :type Actor%20Object%20Reference) (OtherComp :type Primitive%20Component%20Object%20Reference) (OtherBodyIndex :type Integer) (bFromSweep :type Boolean) (SweepResult :type Hit%20Result%20Structure%20%28by%20ref%29))
  (CallFunction|CheckforRiderFunction OtherActor))

(event Custom|SpawnRideableOverlapCheckSphere
  (bind _returnvalue (AddComponent|AddSphereComponent false (Math|Transform|MakeTransform "0.000000,0.000000,0.000000" "0, 0, 0" "1.000000,1.000000,1.000000")))
  (Development|SetHiddeninGame _returnvalue false false)
  (Rendering|SetVisibility _returnvalue true false)
  (Collision|BindEventtoOnComponentBeginOverlap _returnvalue (delegate Custom|CheckForRider))
  (Collision|BindEventtoOnComponentEndOverlap _returnvalue (delegate Custom|Stop%20Check%20for%20Rider))
  (Components|Sphere|SetSphereRadius _returnvalue 1.2e+03 true))

(event Custom|Stop%20Check%20for%20Rider
  (params (OverlappedComponent :type Primitive%20Component%20Object%20Reference) (OtherActor :type Actor%20Object%20Reference) (OtherComp :type Primitive%20Component%20Object%20Reference) (OtherBodyIndex :type Integer))
  (if (== OtherActor (Variables|Default|GetSpawner))
    (Utilities|Time|ClearandInvalidateTimerbyHandle (Variables|Default|GetShowProjectileTimer))))

(event EventBeginPlay
  (Utilities|FlowControl|Delay 5.0)
  (Variables|Default|SetIsFalling true)
  (Class|PrimitiveComponent|SetConstraintMode (Variables|Default|GetIsland) "None"))

(fn ConstructionScript)

(fn SetIsCircled
  (params (CircleBubble :type Circle%20Bubble%20Object%20Reference))
  (bind _island (Variables|Default|GetIsland))
  (bind _island_2 (Variables|Default|GetIsland))
  (Variables|Default|SetCircleBubble CircleBubble)
  (if (Utilities|IsValid CircleBubble)
    (Class|PrimitiveComponent|SetConstraintMode (Variables|Default|GetIsland) "None")
    (Variables|Default|SetStoredMass (Physics|GetMass (Variables|Default|GetIsland)))
    (Class|PrimitiveComponent|SetLinearDamping _island_2 1.0)
    (Class|PrimitiveComponent|SetMassOverrideinKg _island_2 "None" 0.0 true)
    (Class|CircleBubble|SetBubbleLifespan (Variables|Default|GetCircleBubble) 3e+01)
    (Variables|Default|SetIsFalling false)
    (CallFunction|SpawnRideableOverlapCheckSphere)
    (else
      (Class|PrimitiveComponent|SetLinearDamping _island 0.0001)
      (Class|PrimitiveComponent|SetMassOverrideinKg _island "None" (Variables|Default|GetStoredMass) true)
      (Variables|Default|SetIsFalling true)))
  (return false))

(fn GetLocation
  (return (Transformation|GetActorLocation)))

(fn GetIsValid
  (return (Utilities|IsValid self)))

(fn GetIsCircled
  (return (Variables|Default|GetCircleBubble)))

(fn ApplyForce
  (params (OptionalForce :type Vector :default "0, 0, 0"))
  (if (Utilities|IsValid self)
    (Physics|AddForce (Variables|Default|GetIsland) OptionalForce "None" false)
    (return true)))

(fn CheckforRiderFunction
  (params (OverlapActor :type Actor%20Object%20Reference))
  (if (Utilities|IsValid (Variables|Default|GetCircleBubble))
    (if (== OverlapActor (Variables|Default|GetSpawner))
      (bind _returnvalue (Utilities|Time|SetTimerbyFunctionName 0 "ShowProjectileTest" 1.0 true))
      (Variables|Default|SetShowProjectileTimer _returnvalue))))

(fn ShowProjectileTest
  (bind _spawner (Variables|Default|GetSpawner))
  (bind _riderconnectionpoint (Variables|Default|GetRiderConnectionPoint))
  (bind _spawner_2 (Variables|Default|GetSpawner))
  (bind _returnvalue (Transformation|GetActorLocation _spawner))
  (bind _returnvalue_2 (Transformation|GetWorldLocation _riderconnectionpoint))
  (bind _camera (Variables|/Game/Characters/Wizard/WizardBaseBP.WizardBaseBP_C|GetCamera _spawner_2))
  (bind _returnvalue_3 (Transformation|GetWorldRotation _camera))
  (bind _returnvalue_4 (- _returnvalue_2 _returnvalue))
  (bind _returnvalue_5 (Math|Vector|Normalize _returnvalue_4))
  (Development|PrintString (Utilities|String|ToString(Float) 0.0))
  (if (> (Math|Vector|DotProduct (Math|Vector|Normalize (- (Transformation|GetWorldLocation (Variables|Default|GetRiderConnectionPoint)) (Transformation|GetActorLocation _spawner_2))) (Math|Vector|GetForwardVector (Math|Rotator|MakeRotator (.roll _returnvalue_3) (.pitch _returnvalue_3) (.yaw _returnvalue_3)))) 0.5)
    (bind _outhit (Class|GameplayStatics|BlueprintPredictProjectilePathbyTraceChannel _returnvalue (Math|Vector|MakeVector (* (.x _returnvalue_5) 2.5e+02) (* (.y _returnvalue_5) 2.5e+02) (* (.z _returnvalue_5) 1.2e+03)) true 1.0 "ECC_GameTraceChannel3" false (Utilities|Array|MakeArray (Variables|Default|GetSpawner)) "ForDuration" 2.0))
    (Development|PrintString (Utilities|GetDisplayName (.hitcomponent _outhit)))))
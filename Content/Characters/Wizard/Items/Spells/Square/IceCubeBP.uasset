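; Wizard ice wall spell that sizes a destructible barrier to fit the surrounding space.
; Raycast line-traces along the caster's up and right axes to size the box, derive health (lower when larger) and charge mana.
; A looping timer rotates, then moves and scales the wall into place; unfinished walls expire.
; Hits lower health, with projectile overlaps updating a dynamic material and Damage spawning an impulse-driven geometry collection on death.
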(event OnComponentBeginOverlap(Box)
  (params (OverlappedComponent :type Primitive%20Component%20Object%20Reference) (OtherActor :type Actor%20Object%20Reference) (OtherComp :type Primitive%20Component%20Object%20Reference) (OtherBodyIndex :type Integer) (bFromSweep :type Boolean) (SweepResult :type Hit%20Result%20Structure%20%28by%20ref%29))
  (bind _asprojectile_hit_box (Utilities|Casting|CastToProjectileHitBox OtherActor))
  (Default|Destroy _asprojectile_hit_box)
  (CallFunction|DecrementHealth 1e+01))

(event OnComponentEndOverlap(Box)
  (params (OverlappedComponent :type Primitive%20Component%20Object%20Reference) (OtherActor :type Actor%20Object%20Reference) (OtherComp :type Primitive%20Component%20Object%20Reference) (OtherBodyIndex :type Integer)))

(event Custom|Raycast
  (bind _defaultcubesize (Variables|Default|GetDefaultCubeSize))
  (bind _box (Variables|Default|GetBox))
  (bind _forwardvector (Variables|Default|GetForwardVector))
  (bind _box_2 (Variables|Default|GetBox))
  (bind _returnvalue (Transformation|GetWorldRotation _forwardvector))
  (bind _returnvalue_2 (Components|Box|GetScaledBoxExtent _box_2))
  (bind _returnvalue_3 (/ (.x _returnvalue_2) 96.0))
  ;[1 1 1] Init Scale
  (Transformation|SetWorldScale3D (Variables|Default|GetWall) (Math|Vector|MakeVector _returnvalue_3 _returnvalue_3 (/ (.y _returnvalue_2) 96.0)))
  ;[1 1 1] Rotate Raycast Dirs to Player Forward Vec
  (Transformation|SetWorldRotation (Variables|Default|GetForwardVector) (Transformation|GetWorldRotation (Variables|/Script/Engine.Character|GetCapsuleComponent (Variables|Default|GetSpawner))) false false)
  ;[1 1 1] Do Raycast to Surroundings
  (bind (__ishit _hitlength _hitmidpoint _nohitlength _nohitmidpoint) (CallFunction|GetLineMidpointandLength (Math|Vector|GetUpVector (Variables|Default|GetForwardVector)) false))
  (if __ishit
    (Variables|Default|SetVerticalMidpoint _hitmidpoint)
    (Variables|Default|SetHeight _hitlength)
    (else
      (Variables|Default|SetVerticalMidpoint _nohitmidpoint)
      (Variables|Default|SetHeight _nohitlength)))
  (bind (__ishit_2 _hitlength_2 _hitmidpoint_2 _nohitlength_2 _nohitmidpoint_2) (CallFunction|GetLineMidpointandLength (Math|Vector|GetRightVector (Variables|Default|GetForwardVector)) true))
  (if __ishit_2
    (Variables|Default|SetHorizontalMidpoint _hitmidpoint_2)
    (Variables|Default|SetWidth _hitlength_2)
    (else
      (Variables|Default|SetHorizontalMidpoint _nohitmidpoint_2)
      (Variables|Default|SetWidth _nohitlength_2)))
  ;[1 1 1] error
  (if (or (< (Variables|Default|GetWidth) 5.0) (< (Variables|Default|GetHeight) 5.0))
    (Actor|DestroyActor)
    (else
      ;[1 1 1] Set Collision Box Extents from Raycast
      (Components|Box|SetBoxExtent _box (Math|Vector|MakeVector (Variables|Default|GetHeight) (Variables|Default|GetWidth) (Variables|Default|GetDefaultCubeSize)) true)
      ;[1 1 1] Move Collision Box to Center And Rotate to Player's Rot
      (Transformation|SetWorldLocationAndRotation _box (Math|Vector|FindClosestPointonLine (Variables|Default|GetHorizontalMidpoint) (Variables|Default|GetVerticalMidpoint) (Math|Vector|GetRightVector (Variables|Default|GetForwardVector))) (Math|Rotator|MakeRotator (.roll _returnvalue) 9e+01 (.yaw _returnvalue)) false false)
      (Variables|Default|SetDesiredPlaneRotation (Math|Rotator|MakeRotator (.roll _returnvalue) 9e+01 (.yaw _returnvalue)))
      ;[1 1 1] Set Desired Plane scale
      (Variables|Default|SetDesiredPlaneScale (Math|Vector|MakeVector (/ (Variables|Default|GetHeight) _defaultcubesize) (/ (Variables|Default|GetWidth) _defaultcubesize) (/ _defaultcubesize _defaultcubesize)))
      (Variables|Default|SetDesiredPlaneLocation (Math|Vector|FindClosestPointonLine (Variables|Default|GetHorizontalMidpoint) (Variables|Default|GetVerticalMidpoint) (Math|Vector|GetRightVector (Variables|Default|GetForwardVector))))
      (bind _output_get (Variables|Default|SetBarrierHealth (/ (- 5e+03 (+ (Variables|Default|GetHeight) (Variables|Default|GetWidth))) 5e+01)))
      (Default|DecrementMana (Variables|Default|GetSpawner) (+ (/ _output_get 7.0) 0.0))
      (bind _returnvalue_4 (Rendering|Material|CreateDynamicMaterialInstance (Rendering|Material|GetMaterial (Variables|Default|GetWall) 0) "None" "None" :!class /Script/Engine.KismetMaterialLibrary))
      (bind _output_get_2 (Variables|Default|SetDynamicMaterial _returnvalue_4))
      (Rendering|Material|SetMaterial (Variables|Default|GetWall) 0 _output_get_2)
      (Rendering|Material|SetScalarParameterValue _output_get_2 "BarrierHealth" (Math|Float|Clamp(Float) (/ (Variables|Default|GetBarrierHealth) 1e+02) 0.1) :!class /Script/Engine.MaterialInstanceDynamic)
      (bind _returnvalue_5 (Utilities|Time|SetTimerbyFunctionName 0 "InterpPlaneToDesired" 0.05 true 0.5 0.3))
      (Variables|Default|SetInterpTimer _returnvalue_5))))

(event EventBeginPlay
  (Utilities|FlowControl|Delay 8.0)
  (if (not (Variables|Default|GetIsDone))
    (Actor|DestroyActor)))

(event EventSetDoorableWorldLocation
  (params (OptionalLocation :type Vector :default "0, 0, 0")))

(fn ConstructionScript)

(fn GetLineMidpointandLength
  (params (Direction :type Vector) (NeedsBoth :type Boolean))
  (bind _returnvalue (Transformation|GetActorLocation))
  (bind _returnvalue_2 (Transformation|GetActorLocation))
  (bind _defaultcubesize (Variables|Default|GetDefaultCubeSize))
  (bind _returnvalue_3 (* _defaultcubesize -1.0))
  (bind _returnvalue_4 (* Direction _defaultcubesize))
  (bind _returnvalue_5 (+ _returnvalue _returnvalue_4))
  (bind _returnvalue_6 (* Direction _returnvalue_3))
  (bind _returnvalue_7 (+ _returnvalue _returnvalue_6))
  (bind _returnvalue_8 (- _returnvalue_5 _returnvalue_7))
  (bind _outhit (Collision|LineTraceByChannel _returnvalue_2 (+ _returnvalue_2 (* Direction (Variables|Default|GetRaycastDist))) "TraceTypeQuery2" false 0 "ForDuration"))
  (LocalVariables|SetHitLoc1 (.location _outhit))
  (bind _output_get (LocalVariables|SetIsHit (.bblockinghit _outhit)))
  (if _output_get
    _
    (else
      (LocalVariables|SetHitLoc1 _returnvalue_5)))
  (bind _outhit_2 (Collision|LineTraceByChannel _returnvalue_2 (+ _returnvalue_2 (* Direction (* (Variables|Default|GetRaycastDist) -1.0))) "TraceTypeQuery2" false 0 "ForDuration"))
  (if (.bblockinghit _outhit_2)
    _
    (else
      (LocalVariables|SetHitLoc2 _returnvalue_7)))
  (LocalVariables|SetHitLoc2 (.location _outhit_2))
  (if NeedsBoth
    (LocalVariables|SetIsHit (and (.bblockinghit _outhit_2) (LocalVariables|GetIsHit)))
    (else
      (LocalVariables|SetIsHit (or (.bblockinghit _outhit_2) (LocalVariables|GetIsHit)))))
  (return (LocalVariables|GetIsHit) (Math|Vector|Distance(Vector) (LocalVariables|GetHitLoc2) (LocalVariables|GetHitLoc1)) (+ (LocalVariables|GetHitLoc2) (* (Math|Vector|Normalize (- (LocalVariables|GetHitLoc1) (LocalVariables|GetHitLoc2))) (/ (Math|Vector|VectorLength (- (LocalVariables|GetHitLoc1) (LocalVariables|GetHitLoc2))) 2.0))) (Math|Vector|Distance(Vector) _returnvalue_5 _returnvalue_7) (+ _returnvalue_7 (* (Math|Vector|Normalize _returnvalue_8) (/ (Math|Vector|VectorLength _returnvalue_8) 2.0)))))

(fn DecrementHealth
  (params (DmgAmt :type Float%20%28double-precision%29))
  (bind _output_get (Variables|Default|SetBarrierHealth (- (Variables|Default|GetBarrierHealth) DmgAmt)))
  (Development|PrintString (Utilities|String|ToString(Float) (Math|Float|Clamp(Float) (/ _output_get 1e+02) 0.1)))
  (Rendering|Material|SetScalarParameterValue (Variables|Default|GetDynamicMaterial) "BarrierHealth" (Math|Float|Clamp(Float) (/ _output_get 1e+02) 0.1) :!class /Script/Engine.MaterialInstanceDynamic)
  (if (< (Variables|Default|GetBarrierHealth) 0.0)
    (Actor|DestroyActor)))

(fn InterpPlanetoDesired
  (bind _returnvalue (Utilities|Time|GetWorldDeltaSeconds))
  (bind _wall (Variables|Default|GetWall))
  (bind _wall_2 (Variables|Default|GetWall))
  (if (Variables|Default|GetIsRotated)
    (Transformation|SetWorldTransform _wall (Math|Transform|MakeTransform (Math|Interpolation|VInterpTo (Transformation|GetWorldLocation _wall) (Variables|Default|GetDesiredPlaneLocation) _returnvalue 5.0) (Math|Interpolation|RInterpTo (Transformation|GetWorldRotation _wall) (Variables|Default|GetDesiredPlaneRotation) _returnvalue 1e+01) (Math|Interpolation|VInterpTo (Transformation|GetWorldScale _wall) (Variables|Default|GetDesiredPlaneScale) _returnvalue 5.0)) false false)
    (if (Class|KismetMathLibrary|NearlyEqualTransformTransform (Transformation|GetWorldTransform (Variables|Default|GetWall)) (Math|Transform|MakeTransform (Variables|Default|GetDesiredPlaneLocation) (Variables|Default|GetDesiredPlaneRotation) (Variables|Default|GetDesiredPlaneScale)) 2.0 2.0 0.0)
      (Variables|Default|SetIsDone true)
      (Development|PrintString "INTERP")
      (Utilities|Time|ClearandInvalidateTimerbyHandle (Variables|Default|GetInterpTimer))
      (Components|DestroyComponent (Variables|Default|GetNiagara9)))
    (else
      (Transformation|SetWorldTransform _wall_2 (Math|Transform|MakeTransform (Transformation|GetWorldLocation _wall_2) (Math|Interpolation|RInterpTo (Transformation|GetWorldRotation _wall_2) (Variables|Default|GetDesiredPlaneRotation) (Utilities|Time|GetWorldDeltaSeconds) 1e+01) (Transformation|GetWorldScale _wall_2)) false false)
      (if (Utilities|Operators|EqualEqual (Transformation|GetWorldRotation (Variables|Default|GetWall)) (Variables|Default|GetDesiredPlaneRotation) 2.0)
        (Variables|Default|SetIsRotated true)))))

(fn GetHealth
  (if (Utilities|IsValid self)
    (return (Variables|Default|GetBarrierHealth))))

(fn Damage
  (params (dmgAmt :type Float%20%28single-precision%29))
  (if (Utilities|IsValid self)
    (bind _output_get (Variables|Default|SetBarrierHealth (- (Variables|Default|GetBarrierHealth) dmgAmt)))
    (Development|PrintString (Utilities|String|ToString(Float) _output_get))
    (if (<= _output_get 0.0)
      (bind _returnvalue (Game|SpawnActorfromClass "/Game/Characters/Wizard/Items/Spells/Square/IceCubeTEST_GeometryCollection_Blueprint.IceCubeTEST_GeometryCollection_Blueprint_C" (Transformation|GetWorldTransform (Variables|Default|GetWall)) "Undefined" "MultiplyWithRoot" 0 0))
      (Physics|AddImpulse (Variables|/Script/GeometryCollectionEngine.GeometryCollectionActor|GetGeometryCollectionComponent _returnvalue) (Variables|Default|GetHitImpulse) "None" true)
      (Actor|DestroyActor))
    (return true)))

(fn SpawnHitParticle
  (params (Particle :type Niagara%20System%20Object%20Reference) (HitNormal :type Vector :default "0, 0, 0") (Location :type Vector :default "0, 0, 0"))
  (bind _returnvalue (+ Location HitNormal))
  (bind _returnvalue_2 (Math|Rotator|FindLookatRotation Location _returnvalue))
  (if (Utilities|IsValid self)
    (if (Utilities|IsValid Particle)
      (Niagara|SpawnSystematLocation Particle Location _returnvalue_2 "0.300000,0.300000,0.300000"))
    (Niagara|SpawnSystematLocation (Variables|Default|GetHitParticle) Location _returnvalue_2 "0.300000,0.300000,0.300000")
    (return false)))

(fn ApplyHitImpulse
  (params (Impulse :type Vector :default "0, 0, 0"))
  (Variables|Default|SetHitImpulse Impulse)
  (return true))

(fn GetDoorableBounds
  (return (.BoxExtent (Collision|GetComponentBounds (Variables|Default|GetBox)))))

(fn GetDoorableWorldRotation
  (return (Transformation|GetWorldRotation (Variables|Default|GetBox))))

(fn GetDoorableWorldLocation
  (return (.Origin (Collision|GetComponentBounds (Variables|Default|GetBox)))))
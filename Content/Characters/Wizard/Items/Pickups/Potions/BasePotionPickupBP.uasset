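; Base actor for wizard potion pickups, leaving the CompletePickup effect to subclasses.
; Overlapping wizards start a looping timer that retries until the wizard is free, then registers the pickup and destroys it shortly after; leaving cancels it.
; Targeting functions expose location and a proximity-based weight.
; CircleBubble functions alter the physics box's damping and mass, with upward force shared across the bubble's circled objects.
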(event OnComponentBeginOverlap(OverlapSphere)
  (params (OverlappedComponent :type Primitive%20Component%20Object%20Reference) (OtherActor :type Actor%20Object%20Reference) (OtherComp :type Primitive%20Component%20Object%20Reference) (OtherBodyIndex :type Integer) (bFromSweep :type Boolean) (SweepResult :type Hit%20Result%20Structure%20%28by%20ref%29))
  (bind _aswizard_base_bp (Utilities|Casting|CastToWizardBaseBP OtherActor))
  (Variables|Default|SetPlayerPickingup _aswizard_base_bp)
  (bind _returnvalue (Utilities|Time|SetTimerbyEvent (delegate Custom|BeginPickup) 0.7 true))
  (Variables|Default|SetPickupTimer _returnvalue))

(event OnComponentEndOverlap(OverlapSphere)
  (params (OverlappedComponent :type Primitive%20Component%20Object%20Reference) (OtherActor :type Actor%20Object%20Reference) (OtherComp :type Primitive%20Component%20Object%20Reference) (OtherBodyIndex :type Integer))
  (bind _aswizard_base_bp (Utilities|Casting|CastToWizardBaseBP OtherActor))
  (if (and (== _aswizard_base_bp (Variables|Default|GetPlayerPickingup)) (Utilities|IsValid (Variables|Default|GetOverlapSphere)))
    (Utilities|Time|ClearandInvalidateTimerbyHandle (Variables|Default|GetPickupTimer))
    (Variables|Default|SetPlayerPickingup 0)))

(event Custom|BeginPickup
  (bind _playerpickingup (Variables|Default|GetPlayerPickingup))
  (bind _playerpickingup_2 (Variables|Default|GetPlayerPickingup))
  (if (Utilities|IsValid _playerpickingup)
    (if (not (Variables|/Game/Characters/Wizard/WizardBaseBP.WizardBaseBP_C|GetIsPickup _playerpickingup))
      (Variables|/Game/Characters/Wizard/WizardBaseBP.WizardBaseBP_C|SetIsPickup _playerpickingup_2 true)
      (Default|ToggleonActive _playerpickingup_2)
      (Variables|/Game/Characters/Wizard/WizardBaseBP.WizardBaseBP_C|SetPickupRef _playerpickingup_2 self)
      (Utilities|Time|ClearandInvalidateTimerbyHandle (Variables|Default|GetPickupTimer))
      (Utilities|FlowControl|Delay 0.55)
      (Actor|DestroyActor))))

(event Custom|CompletePickup
  ;[1 1 1] ForSubClasses
)

(event EventBeginPlay)

(event Collision|EventActorBeginOverlap
  (params (OtherActor :type Actor%20Object%20Reference)))

(event EventTick
  (params (DeltaSeconds :type Float%20%28single-precision%29)))

(fn ConstructionScript)

(fn GetWeight
  (params (Caller :type Actor%20Object%20Reference))
  (bind _returnvalue (Transformation|GetActorLocation))
  (bind _returnvalue_2 (Transformation|GetActorLocation Caller))
  (bind _returnvalue_3 (Math|Vector|Distance(Vector) _returnvalue_2 _returnvalue))
  (if (< _returnvalue_3 1e+03)
    (LocalVariables|SetWeight (Math|Float|Truncate (Math|Float|MapRangeClamped _returnvalue_3 0.0 1e+03 5.0 1.0)))
    (else
      (LocalVariables|SetWeight 0)))
  (return (LocalVariables|GetWeight)))

(fn GetLocation
  (return (+ (Transformation|GetActorLocation) "0.000000,0.000000,10.000000")))

(fn ApplyImpulse
  (params (Impulse :type Vector :default "0, 0, 0"))
  (Physics|AddImpulse (Variables|Default|GetBox) Impulse "None" false)
  (return true))

(fn ApplyForce
  (if (Utilities|IsValid self)
    (Physics|AddForce (Variables|Default|GetBox) (Math|Vector|MakeVector 0.0 0.0 (Math|Float|SafeDivide 1e+03 (Math|Conversions|ToFloat(Integer) (Utilities|Array|Length (Variables|/Script/BattleWizard.CircleBubble|GetCircleables (Variables|Default|GetCircleBubble)))))) "None" false)
    (return true)))

(fn GetIsValid
  (return (Utilities|IsValid self)))

(fn SetIsCircled
  (params (CircleBubble :type Circle%20Bubble%20Object%20Reference))
  (Variables|Default|SetCircleBubble CircleBubble)
  (if (Utilities|IsValid CircleBubble)
    (Class|PrimitiveComponent|SetLinearDamping (Variables|Default|GetBox) 1.0)
    (Class|PrimitiveComponent|SetMassOverrideinKg (Variables|Default|GetBox) "None" 0.0 true)
    (else
      (Class|PrimitiveComponent|SetLinearDamping (Variables|Default|GetBox) 0.0001)
      (Class|PrimitiveComponent|SetMassOverrideinKg (Variables|Default|GetBox) "None" 1.0 true)))
  (return true))

(fn GetIsCircled
  (return (Variables|Default|GetCircleBubble)))

(fn GetTargetLocation
  (if (Utilities|IsValid self)
    (return (Transformation|GetActorLocation))))